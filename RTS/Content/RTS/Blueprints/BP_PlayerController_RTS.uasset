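; RTS camera Blueprint that pans, zooms and rotates the view through a spring arm and floating pawn movement.
; IA_Move drives movement along the camera's right and forward vectors, flattened to the ground plane.
; Each tick, zoom and rotate inputs are lerp-smoothed into rates that change clamped arm length and arm yaw.
; Maximum pan speed scales with arm length, so movement is faster when zoomed out.
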(event `self.ReceiveTick`
  (params (DeltaSeconds :type "Float (single-precision)"))
  (`self.Camera Zoom`)
  (`self.RotateCamera`))

(event `EnhancedInput|/Game/RTS/Input/Actions/IA_Move`
  (params (ActionValue :type "Vector2D Structure") (ElapsedSeconds :type "Float (double-precision)") (TriggeredSeconds :type "Float (double-precision)") (InputAction :type "InputAction Object Reference" :default "/Game/RTS/Input/Actions/IA_Move.IA_Move"))
  (bind (_returnvalue_x _returnvalue_y) (`KismetMathLibrary.BreakVector` (`SceneComponent.GetForwardVector` (`self.Camera`))))
  (bind (_returnvalue_x_2 _returnvalue_y_2) (`KismetMathLibrary.BreakVector` (`SceneComponent.GetRightVector` (`self.Camera`))))
  (:`Triggered`
    (`self.AddMovementInput` (`KismetMathLibrary.Normal` (`KismetMathLibrary.MakeVector` _returnvalue_x_2 _returnvalue_y_2)) ActionValue_X)
    (`self.AddMovementInput` (`KismetMathLibrary.Normal` (`KismetMathLibrary.MakeVector` _returnvalue_x _returnvalue_y)) ActionValue_Y)))

(fn `Camera Zoom`
  (bind _springarm (`self.SpringArm`))
  (bind _output_get (set `self.ZoomRate` (`KismetMathLibrary.Lerp` (`self.ZoomRate`) (* (`|GetInputActionValue`) -100.0) (* (`GameplayStatics.GetWorldDeltaSeconds`) 10.0))))
  (bind _output_get_2 (set `SpringArmComponent.TargetArmLength` (`KismetMathLibrary.FClamp` (+ (`SpringArmComponent.TargetArmLength` _springarm) _output_get) 500.0 10000.0) _springarm))
  (set `FloatingPawnMovement.MaxSpeed` (/ _output_get_2 2.0) (`self.FloatingPawnMovement`)))

(fn `RotateCamera`
  (bind _output_get (set `self.RotationRate` (`KismetMathLibrary.Lerp` (`self.RotationRate`) (* (`|GetInputActionValue`) 2.5) (* (`GameplayStatics.GetWorldDeltaSeconds`) 5.0))))
  (`SceneComponent.K2_AddRelativeRotation` (`self.SpringArm`) (`KismetMathLibrary.MakeRotator` 0.0 0.0 _output_get) false false))

(fn `UserConstructionScript`)